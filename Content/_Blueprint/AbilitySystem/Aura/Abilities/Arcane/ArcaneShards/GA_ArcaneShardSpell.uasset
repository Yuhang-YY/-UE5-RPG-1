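; Gameplay ability for the Arcane Shards spell, which erupts a series of damaging shards around a targeted ground location.
; Activation shows a magic circle; an input press captures the cursor hit, spawns BP_PointCollection for ground points and plays the cast montage.
; The montage's gameplay event starts a looping timer that, per point, damages nearby living actors and fires the shard GameplayCue.
; After the last point, it destroys the collection and ends the ability.
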(event `self.K2_ActivateAbility`
  (`|ExecutionSequence`
    (:`then_0`
      ;[1 0.2911 0.2812] 显示魔法阵
      (message `PlayerInterface.ShowMagicCircleDecal` (`self.GetAvatarActorFromActorInfo`) null))
    (:`then_1`
      (`AbilityTask_WaitInputPress.WaitInputPress` false
        (:`OnPress`
          ;[1 0.9238 0.3] 获取鼠标移动位置
          (bind (_asynctaskproxy _datahandle) (`TargetDataUnderMouse.CreateTargetDataUnderMouse` null)
            (:`DataValid`
              (set `self.MouseHitLocation` (`.ImpactPoint` (`GameplayStatics.BreakHitResult` (`AbilitySystemBlueprintLibrary.GetHitResultFromTargetData` _datahandle))))
              (`|ExecutionSequence`
                (:`then_0`
                  ;[0.2443 1 0.2126] SpawnPoint Collection And Get Ground Point
                  (bind _returnvalue (`|SpawnActorFromClass` "/Game/_Blueprint/AbilitySystem/Aura/Abilities/Arcane/ArcaneShards/BP_PointCollection.BP_PointCollection_C" (`KismetMathLibrary.MakeTransform` (`self.MouseHitLocation`)) "AlwaysSpawn" "MultiplyWithRoot" null null))
                  (bind _output_get (set `self.PointCollection` _returnvalue))
                  (set `self.GroundPoints` (`PointCollection.GetGroundPoints` _output_get (`self.MouseHitLocation`) (`self.NumPoints`) 0.0)))
                (:`then_1`
                  ;[0.9074 0.1602 1] UpdateFacingTarget
                  (message `CombatInterface.UpdateFacingTarget` (`self.GetAvatarActorFromActorInfo`) (`self.MouseHitLocation`)))
                (:`then_2`
                  ;[1 0.1458 0.1458] 播放蒙太奇动画等待标签事件
                  (`AbilityTask_PlayMontageAndWait.CreatePlayMontageAndWaitProxy` "None" "/Game/Assets/Characters/Aura/Animations/Abilities/AM_Cast_ArcaneShards.AM_Cast_ArcaneShards"
                    (:`then`
                      (`AbilityTask_WaitGameplayEvent.WaitGameplayEvent` (struct :`TagName` "Event.Montage.ArcaneShard") null true
                        (:`EventReceived`
                          (bind _returnvalue_2 (`KismetSystemLibrary.K2_SetTimerDelegate` (delegate `显示ArcaneShard`) (`self.ShardSpawnDeltaTime`) true))
                          (set `self.TimerHandle` _returnvalue_2)
                          (`self.显示ArcaneShard`)
                          (message `PlayerInterface.HideMagicCircleDecal` (`self.GetAvatarActorFromActorInfo`)))))))))))))))

(event `显示ArcaneShard`
  (if (< (`self.count`) (`self.NumPoints`))
    (`self.存储碎片生成位置`)
    (bind _output_get (`self.检测附近的敌人`))
    (for _array_element _output_get
      (`self.对敌人造成伤害` _array_element))
    (`/Engine/EditorBlueprintResources/StandardMacros.IncrementInt` (`self.count`)
      (:`  `
        (`self.K2_ExecuteGameplayCueWithParams` (struct :`TagName` "GameplayCue.ArcaneShards") (`AbilitySystemBlueprintLibrary.MakeGameplayCueParameters` 0.0 0.0 (struct) (struct) (struct) (struct) (struct) (`self.SpawnLocation`)))))
    (else
      (`KismetSystemLibrary.K2_ClearAndInvalidateTimerHandle` (`self.TimerHandle`))
      (`KismetSystemLibrary.Delay` 0.2)
      (`Actor.K2_DestroyActor` (`self.PointCollection`))
      (`self.K2_EndAbility`))))

(fn `存储碎片生成位置`
  (set `self.SpawnLocation` (`SceneComponent.K2_GetComponentLocation` (`|GetArrayItem` (`self.GroundPoints`) (`self.count`)))))

(fn `对敌人造成伤害`
  (params (Target :type "Actor Object Reference"))
  (`AuraWidgetControllerLibrary.ApplyDamageEffect` (`self.MakeDamageEffectParamsFromClassDefaults` Target (`self.SpawnLocation`))))

(fn `检测附近的敌人`
  (returns (Output_Get :type "Array of Actor Object Reference"))
  (bind _returnvalue (`self.GetAvatarActorFromActorInfo`))
  (bind _outactors (`AuraWidgetControllerLibrary.GetLifeActorWithingRadius` _returnvalue (`|MakeArray` _returnvalue) (`self.RadialDamageOuterRadius`) (`self.SpawnLocation`)))
  (bind _output_get (set `self.OverlappingActor` _outactors))
  (return _output_get))