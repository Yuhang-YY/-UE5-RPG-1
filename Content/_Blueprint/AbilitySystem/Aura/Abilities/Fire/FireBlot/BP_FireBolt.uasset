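; Fire Bolt actor that explodes when it stops moving, apparently the projectile for Aura's fire ability.
; Each Tick it compares its current location with the previous frame's to measure how far it travelled.
; When that distance is at or below MinDistance, it plays the impact sound, spawns the fire explosion effect and destroys itself.
; The graph itself contains no overlap or damage logic.
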(event `self.ReceiveTick`
  (params (DeltaSeconds :type "Float (single-precision)"))
  (bind _currentactorlocation (`self.CurrentActorLocation`))
  (set `self.LastActorLocation` (`self.CurrentActorLocation`))
  (set `self.CurrentActorLocation` (`self.K2_GetActorLocation`))
  (if (<= (`KismetMathLibrary.VSize` (- (`self.LastActorLocation`) (`self.CurrentActorLocation`))) (`self.MinDistance`))
    (`GameplayStatics.SpawnSoundAtLocation` "/Game/Assets/Sounds/Abilities/FireBolt/sfx_FireBolt_Impact.sfx_FireBolt_Impact" _currentactorlocation (struct) 1.0 1.0 0.0 null null)
    (`NiagaraFunctionLibrary.SpawnSystemAtLocation` "/Game/Assets/Effects/Projectiles/FireExplosion/NS_FireExplosion.NS_FireExplosion" _currentactorlocation)
    (`self.K2_DestroyActor`)))

(fn `UserConstructionScript`)