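; GA_Fire is the fire bolt gameplay ability that casts projectiles toward the target under the mouse.
; On activation it commits, reads the cursor hit through a target data task, turns the avatar toward it via CombatInterface and plays the cast montage.
; The montage's gameplay event spawns projectiles from the weapon socket with an overridden pitch and the hit actor as homing target, and montage completion ends the ability.
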(event `self.K2_ActivateAbility`
  (bind _returnvalue (`self.K2_CommitAbility`))
  (if _returnvalue
    (bind (_asynctaskproxy _datahandle) (`TargetDataUnderMouse.CreateTargetDataUnderMouse` null)
      (:`DataValid`
        (bind (_bblockinghit _binitialoverlap _time _distance _location _impactpoint _normal _impactnormal _physmat _hitactor) (`GameplayStatics.BreakHitResult` (`AbilitySystemBlueprintLibrary.GetHitResultFromTargetData` _datahandle)))
        (set `self.Location` _location)
        (set `self.Hit Actor` _hitactor)
        (bind _ascombat_interface (cast `CombatInterface` (`self.GetAvatarActorFromActorInfo`)))
        (`CombatInterface.UpdateFacingTarget` _ascombat_interface (`self.Location`))
        (`AbilityTask_PlayMontageAndWait.CreatePlayMontageAndWaitProxy` "None" "/Game/Assets/Characters/Aura/Animations/Abilities/Am_MyFireBolt.Am_MyFireBolt" 1.0 "None" false
          (:`then`
            (`AbilityTask_WaitGameplayEvent.WaitGameplayEvent` (struct :`TagName` "Event.Montage.FireBolt") null
              (:`EventReceived`
                (`self.SpawnProjectiles` (`self.Location`) (`BlueprintGameplayTagLibrary.MakeLiteralGameplayTag` (struct :`TagName` "CombatSocket.Weapon")) true 45.0 (`self.Hit Actor`)))))
          (:`OnCompleted`
            (`self.K2_EndAbility`)))))))