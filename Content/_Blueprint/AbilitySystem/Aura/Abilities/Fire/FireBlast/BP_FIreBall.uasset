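; Boomerang fireball actor for the Fire Blast ability that flies out, returns and explodes.
; On authority, one timeline lerps it forward, then a second lerps it back toward the moving ReturnActor, both without sweep.
; Once within the minimum explosion distance, it calls OnHit, gathers nearby live actors, applies ExplosiveParams as radial damage to those with an Ability System Component, and destroys itself.
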(event `self.StartOutgoingTimeline`
  (bind _array (`|MakeArray` (`self.GetOwner`) null))
  (`/Engine/EditorBlueprintResources/ActorMacros.Switch Has Authority`
    (:`Authority`
      (set `self.CurrentLocation` (`self.K2_GetActorLocation`))
      (set `self.UpdateLocation` (+ (`self.K2_GetActorLocation`) (* (`self.GetActorForwardVector`) (`self.TraceInstance`))))
      (bind (_direction `_新建轨道_0`) (`Timeline|火球出发`)
        (:`Update`
          (`self.K2_SetActorLocation` (`KismetMathLibrary.VLerp` (`self.CurrentLocation`) (`self.UpdateLocation`) `_新建轨道_0`)))
        (:`Finished`
          (bind (_direction_2 `_新建轨道_0_2`) (`Timeline|返回火球`)
            (:`Update`
              (`self.K2_SetActorLocation` (`KismetMathLibrary.VLerp` (`self.UpdateLocation`) (`self.K2_GetActorLocation` (`self.ReturnActor`)) `_新建轨道_0_2`))
              (if (`self.是否进入爆炸范围`)
                (`self.OnHit`)
                (`KismetArrayLibrary.Array_Add` _array self)
                (bind _outactors (`AuraWidgetControllerLibrary.GetLifeActorWithingRadius` self _array 300.0 (`self.K2_GetActorLocation`)))
                (set `self.Out Actors` _outactors)
                (`AuraWidgetControllerLibrary.SetIsRadialDamageEffectParams` (`self.ExplosiveParams`) true 50.0 300.0 (`self.K2_GetActorLocation`))
                (for _array_element (`self.Out Actors`)
                  (bind _returnvalue (`AbilitySystemBlueprintLibrary.GetAbilitySystemComponent` _array_element))
                  (`/Engine/EditorBlueprintResources/StandardMacros.IsValid` _returnvalue
                    (:`Is Valid`
                      (`AuraWidgetControllerLibrary.SetDamageEffectParamForTargetASC` (`self.ExplosiveParams`) _returnvalue)
                      (`AuraWidgetControllerLibrary.ApplyDamageEffect` (`self.ExplosiveParams`)))))
                (`self.K2_DestroyActor`)))))))))

(fn `UserConstructionScript`)

(fn `是否进入爆炸范围`
  (returns (ReturnValue :type Boolean))
  (return (<= (`KismetMathLibrary.VSize` (- (`self.K2_GetActorLocation`) (`self.K2_GetActorLocation` (`self.ReturnActor`)))) (`self.最小爆炸距离`))))