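; BP_EnemyBase is an enemy base Blueprint that handles the cosmetic spawn scale, facing target and dissolve effects.
; On BeginPlay, the ScaleSpawn timeline animates the mesh's relative scale uniformly.
; UpdateFacingTarget feeds a location to the MotionWarping component as the FacingTarget warp target.
; Separate actor and weapon dissolve events use their own timelines to drive the DisSolve scalar on the dynamic material instance passed in.
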(event `self.ReceiveBeginPlay`
  (bind (_direction _scalefloat) (`Timeline|scaleSpawn`)
    (:`Update`
      (`SceneComponent.SetRelativeScale3D` (`self.Mesh`) (`KismetMathLibrary.MakeVector` _scalefloat _scalefloat _scalefloat)))))

(event `CombatInterface.UpdateFacingTarget`
  (params (Target :type "Vector Structure (by ref)"))
  (`MotionWarpingComponent.AddOrUpdateWarpTargetFromLocation` (`self.MotionWarping`) "FacingTarget" Target))

(event `self.StartActorDisSolveTimeLine`
  (params (MaterialInstanceDynamic :type "MaterialInstanceDynamic Object Reference"))
  (bind (_direction _dissolve) (`Timeline|溶解时间线`)
    (:`Update`
      (`MaterialInstanceDynamic.SetScalarParameterValue` MaterialInstanceDynamic "DisSolve" _dissolve))))

(event `self.StartWeaponDisSolveTimeLine`
  (params (MaterialInstanceDynamic :type "MaterialInstanceDynamic Object Reference"))
  (bind (_direction _dissolve) (`Timeline|时间轴`)
    (:`Update`
      (`MaterialInstanceDynamic.SetScalarParameterValue` MaterialInstanceDynamic "DisSolve" _dissolve))))

(fn `UserConstructionScript`)